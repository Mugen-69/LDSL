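; BP_Ball is the game ball that players catch, throw, lob, smash, recall and use for a dragon-spawning ultimate.
; Throw, Lob and Smash drive projectile and rotating movement, while Recup lerps the ball back to the hand socket by timeline.
; Overlap auto-catches after a short retriggerable delay unless a right-click smash intervenes.
; Timelines toggle the lock-on marker by player distance and trace downward to place and scale a height-based ground decal.
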(event `self.ReceiveTick`
  (params (DeltaSeconds :type "Float (single-precision)"))
  ;[1 1 1] Test state
)

(event `Ball is in the air`
  (bind _balldistancetotheground (`self.BallDistanceToTheGround`))
  ;[1 1 1] Make a timeline that send the raycast event evry 5 seconds
  (`|ExecutionSequence`
    (:`then_0`
      (`/Engine/EditorBlueprintResources/StandardMacros.DoOnce` false :!label _label
        (:`Completed`
          (`SceneComponent.SetVisibility` (`self.ChildActorD_Decal`) true false))))
    (:`then_1`
      (`Timeline|CallRaycastRate` :!via `PlayFromStart` :!label _label_2
        (:`Update`
          (`self.BallHeight`)
          ;[1 1 1] Calculate the size of the ball decal on the ground
          (if (>= _balldistancetotheground 1000.0)
            (`SceneComponent.SetWorldScale3D` (`self.ChildActorD_Decal`) (* (* (1.0 1.0 1.0) (/ _balldistancetotheground 1000.0)) 0.5))
            (elif (<= (`self.BallDistanceToTheGround`) 200.0)
              (`SceneComponent.SetWorldScale3D` (`self.ChildActorD_Decal`) (* (* (1.0 1.0 1.0) (/ 200.0 1000.0)) 0.5))
              (else
                (`SceneComponent.SetWorldScale3D` (`self.ChildActorD_Decal`) (* (* (1.0 1.0 1.0) (/ _balldistancetotheground 1000.0)) 0.5))))))))))

(event `self.ReceiveBeginPlay`
  (bind _lockon (`self.LockOn`))
  ;[1 1 1] Set my variable so the projectile movement doesn't come back to null after it stops
  (`|ExecutionSequence`
    (:`then_0`
      ;[1 1 1] Check the distance between the ball and the player
      (`Timeline|Refresh`
        (:`Update`
          (if (`self.InHand`)
            (`SceneComponent.SetHiddenInGame` (`self.LockOn`) true false)
            (else
              (bind _output_get (set `self.DistanceToBall` (`self.GetDistanceTo` (`self.CharcterBP`))))
              (if (> _output_get 30.0)
                (`SceneComponent.SetHiddenInGame` _lockon false false)
                (else
                  (`SceneComponent.SetHiddenInGame` _lockon true false))))))))
    (:`then_1`
      (set `self.Updated component` (`MovementComponent.UpdatedComponent` (`self.ProjectileMovement`))))
    (:`then_2`
      ;[1 1 1] Initialisation
      (`WidgetComponent.SetTintColorAndOpacity` (`self.LockOn`) (`self.WidgetColor`)))
    (:`then_3`
      (`ActorComponent.Activate` (`self.ProjectileMovement`) true)
      (`PrimitiveComponent.SetCollisionProfileName` (`self.StaticMesh`) "BallThrown" true))))

(event `self.StaticMesh.OnComponentHit`
  (params (HitComponent :type "PrimitiveComponent Object Reference") (OtherActor :type "Actor Object Reference") (OtherComp :type "PrimitiveComponent Object Reference") (NormalImpulse :type "Vector Structure") (Hit :type "HitResult Structure (by ref)"))
  ;[1 1 1] Stop ball rotation when hits the ground
  (if (`self.BallThrown`)
    (`|ExecutionSequence`
      (:`then_0`
        (`self.Stop`))
      (:`then_1`
        (`GameplayStatics.PlaySoundAtLocation` "/Game/Sounds/Ball_Pass_03.Ball_Pass_03" (`SceneComponent.K2_GetComponentLocation` (`self.StaticMesh`)) (struct) 1.0 1.0 0.0 null null null)))))

(event `Ball In the hands`
  ;[1 1 1] Make a timeline that send the raycast event evry 5 seconds
  (`SceneComponent.SetVisibility` (`self.ChildActorD_Decal`) false false)
  (`|ExecutionSequence`
    (:`then_0`
      (goto _label_2 :!via `Stop`))
    (:`then_1`
      (goto _label :!via `Reset`))))

(event `Stop`
  ;[1 1 1] Stop ball rotation when hits the ground
  (`ActorComponent.Deactivate` (`self.RotatingMovement`))
  (set `ProjectileMovementComponent.ProjectileGravityScale` 0.6 (`self.ProjectileMovement`)))

(event `SpecialAbility`
  ;[1 1 1] Utimate
  (`self.Ultimate`)
  (`self.TrailMaxThrow`))

(event `Recup`
  (params (Player :type "/Game/GameMechanics/Character/ThirdPersonCharacter Object Reference"))
  ;[1 1 1] Bring back the ball at it's initial location in the player hands
  (`self.Ball In the hands`)
  (`MovementComponent.SetUpdatedComponent` (`self.ProjectileMovement`) (`self.Updated component`))
  (if (`self.BallThrown`)
    (set `self.BallThrown` false)
    (`PrimitiveComponent.SetCollisionProfileName` (`self.StaticMesh`) "BallInHand" true)
    (`ActorComponent.Deactivate` (`self.ProjectileMovement`))
    (set `self.CallBackInitialLoc` (`self.K2_GetActorLocation`))
    (bind (_direction _factor) (`Timeline|CallBackTimeline` :!via `PlayFromStart`)
      (:`Update`
        (`self.K2_SetActorLocation` (`KismetMathLibrary.VLerp` (`self.CallBackInitialLoc`) (`SceneComponent.GetSocketLocation` (`Character.Mesh` Player) "Ball_socket") _factor) false true))
      (:`Finished`
        (`/Game/GameMechanics/Character/ThirdPersonCharacter.GrabBall` Player self)
        (set `/Game/GameMechanics/Character/ThirdPersonCharacter.Ball` true Player)))))

(event `ThrowBallUlt`
  (bind _projectilemovement (`self.ProjectileMovement`))
  ;[1 1 1] Utimate
  (set `ProjectileMovementComponent.ProjectileGravityScale` 0.0 _projectilemovement)
  (set `MovementComponent.Velocity` (* (`KismetMathLibrary.Normal` (- (`/Game/GameMechanics/Character/ThirdPersonCharacter.CamRay` (`self.CharcterBP`)) (`self.K2_GetActorLocation`))) (`self.SpeedBallUlt`)) _projectilemovement))

(event `self.Trigger_Area.OnComponentBeginOverlap`
  (params (OverlappedComponent :type "PrimitiveComponent Object Reference") (OtherActor :type "Actor Object Reference") (OtherComp :type "PrimitiveComponent Object Reference") (OtherBodyIndex :type Integer) (bFromSweep :type Boolean) (SweepResult :type "HitResult Structure (by ref)"))
  ;[1 1 1] Detects when the player CAN pick up the ball OR smash the ball
  (if (`self.InHand`)
    (`KismetSystemLibrary.PrintString` "Hands full")
    (elif (`self.ActorHasTag` OtherActor "Player")
      (set `self.InArea` true)
      (bind _asthird_person_character (cast `/Game/GameMechanics/Character/ThirdPersonCharacter` OtherActor))
      (set `self.CharcterBP` _asthird_person_character)
      (`KismetSystemLibrary.RetriggerableDelay` 0.15 :!label _label_3)
      (if (stale `RightMouseButtonPressed` _output_get)
        (set `self.Smashed` false)
        (else
          (`/Game/GameMechanics/Character/ThirdPersonCharacter.InBallArea` _asthird_person_character self)
          (set `self.InArea` false)
          (set `self.InHand` true)
          (set `/Game/GameMechanics/Character/ThirdPersonCharacter.InHand` true _asthird_person_character)
          (`self.TrailNormalThrow`)))
      (else
        (set `self.InArea` false)))))

(event `RightMouseButtonPressed`
  ;[1 1 1] Detects when the player CAN pick up the ball OR smash the ball
  (set `self.Smash?` true)
  (if (`self.InArea`)
    (set `self.BallLocation` (`SceneComponent.K2_GetComponentLocation` (`self.StaticMesh`)))
    (if (> (`self.BallDistanceToTheGround`) 140.0)
      (if (not (`self.Smashed`))
        (bind _output_get (set `self.Smashed` true))
        (`|ExecutionSequence`
          (:`then_0`
            (goto _label_3))
          (:`then_1`
            (bind _asthird_person_character (cast `/Game/GameMechanics/Character/ThirdPersonCharacter` (`GameplayStatics.GetPlayerCharacter` 0)))
            (`/Game/GameMechanics/Character/ThirdPersonCharacter.Smash` _asthird_person_character)
            (set `self.InArea` false)
            (`self.BallHeight`)
            (`self.TrailMaxThrow`)))))))

(event `RightMouseButtonReleased`
  ;[1 1 1] Detects when the player CAN pick up the ball OR smash the ball
  (set `self.Smash?` false))

(event `TrailMaxThrow`
  ;[1 1 1] Ball trail colors
  (`NiagaraComponent.SetVariableLinearColor` (`self.Trail`) "User.Color" (make `LinearColor` 0.0 35.0 60.0 60.0)))

(event `TrailNormalThrow`
  ;[1 1 1] Ball trail colors
  (`NiagaraComponent.SetVariableLinearColor` (`self.Trail`) "User.Color" (make `LinearColor` 41.0 57.0 60.0 60.0)))

(event `TP ball center`
  ;[1 1 1] TP the ball in the center
)

(fn `BallFallingTrajectory`)

(fn `BallHeight`
  (bind _returnvalue (`SceneComponent.K2_GetComponentLocation` (`self.StaticMesh`)))
  ;[1 1 1] Calculate the distance ball/ground and set decal location
  (bind _outhit (`KismetSystemLibrary.LineTraceSingle` _returnvalue (- _returnvalue (0.0 0.0 10000.0)) "TraceTypeQuery1"))
  (bind (_bblockinghit _binitialoverlap _time _distance _location _impactpoint) (`GameplayStatics.BreakHitResult` _outhit))
  (set `self.BallDistanceToTheGround` _distance)
  (`self.K2_SetActorLocation` (`ChildActorComponent.ChildActor` (`self.ChildActorD_Decal`)) (`KismetMathLibrary.VLerp` _impactpoint (`self.K2_GetActorLocation` (`ChildActorComponent.ChildActor` (`self.ChildActorD_Decal`))) (`GameplayStatics.GetWorldDeltaSeconds`)) false false))

(fn `Lob`
  (params (Direction :type "Vector Structure"))
  (bind _projectilemovement (`self.ProjectileMovement`))
  (bind _rotatingmovement (`self.RotatingMovement`))
  (`|ExecutionSequence`
    (:`then_0`
      ;[1 1 1] Activate projectile movement and add velocity
      (set `self.LobDirection` Direction)
      (set `self.BallThrown` true)
      (`ActorComponent.Activate` _projectilemovement true)
      (set `MovementComponent.Velocity` (* (`self.LobDirection`) (`self.SpeedLob`)) _projectilemovement)
      (set `self.InHand` false)
      (`self.Ball is in the air`)
      (`GameplayStatics.PlaySoundAtLocation` "/Game/Sounds/Lob.Lob" (`SceneComponent.K2_GetComponentLocation` (`self.StaticMesh`)) (struct) 1.0 1.0 0.0 null null null))
    (:`then_1`
      ;[1 1 1] Rotate the ball on itself after Smash
      (set `RotatingMovementComponent.RotationRate` (`self.LobRotation rate`) _rotatingmovement)
      (`ActorComponent.Activate` _rotatingmovement true)
      (`PrimitiveComponent.SetCollisionProfileName` (`self.StaticMesh`) "BallThrown" true))))

(fn `Smash`
  (params (Destination :type "Vector Structure"))
  (bind _projectilemovement (`self.ProjectileMovement`))
  (bind _rotatingmovement (`self.RotatingMovement`))
  (`|ExecutionSequence`
    (:`then_0`
      ;[1 1 1] Activate projectile movement and add velocity
      (set `self.SmashDirection` (`KismetMathLibrary.Normal` (- Destination (`self.K2_GetActorLocation`))))
      (set `self.BallThrown` true)
      (`ActorComponent.Activate` _projectilemovement true)
      (set `MovementComponent.Velocity` (* (`self.SmashDirection`) (`self.SpeedSmash`)) _projectilemovement)
      (`self.Ball is in the air`)
      (`GameplayStatics.PlaySoundAtLocation` "/Game/Sounds/Smash.Smash" (`SceneComponent.K2_GetComponentLocation` (`self.StaticMesh`)) (struct) 1.0 1.0 0.0 null null null))
    (:`then_1`
      ;[1 1 1] Rotate the ball on itself after Smash
      (set `RotatingMovementComponent.RotationRate` (`self.ThrowRotation rate`) _rotatingmovement)
      (`ActorComponent.Activate` _rotatingmovement true)
      (`PrimitiveComponent.SetCollisionProfileName` (`self.StaticMesh`) "BallThrown" true))))

(fn `Throw`
  (params (Destination :type "Vector Structure"))
  (bind _projectilemovement (`self.ProjectileMovement`))
  (bind _rotatingmovement (`self.RotatingMovement`))
  (`|ExecutionSequence`
    (:`then_0`
      ;[1 1 1] Activate projectile movement and add velocity
      (set `self.BallThrown` true)
      (`ActorComponent.Activate` _projectilemovement true)
      (set `MovementComponent.Velocity` (`/Game/GameMechanics/Character/ThirdPersonCharacter.ThrowVelocity` (`self.CharcterBP`)) _projectilemovement)
      (set `self.InHand` false)
      (`self.Ball is in the air`)
      (set `/Game/GameMechanics/Character/ThirdPersonCharacter.ChargeThrowFloat` 0.0 (`self.CharcterBP`))
      (`GameplayStatics.PlaySoundAtLocation` "/Game/Sounds/WHOOSH_Ball_Crackle_Small_02.WHOOSH_Ball_Crackle_Small_02" (`SceneComponent.K2_GetComponentLocation` (`self.StaticMesh`)) (struct) 1.0 1.0 0.0 null null null))
    (:`then_1`
      ;[1 1 1] Rotate the ball on itself after Throw
      (set `RotatingMovementComponent.RotationRate` (`self.ThrowRotation rate`) _rotatingmovement)
      (`ActorComponent.Activate` _rotatingmovement true)
      (`PrimitiveComponent.SetCollisionProfileName` (`self.StaticMesh`) "BallThrown" true))))

(fn `Ultimate`
  ;[1 1 1] Get the direction of the camera, instantiates the dragon and send the dragon to this direction
  (bind _asthird_person_character (cast `/Game/GameMechanics/Character/ThirdPersonCharacter` (`GameplayStatics.GetPlayerCharacter` 0)))
  (`/Game/GameMechanics/Character/ThirdPersonCharacter.CameraForwardRaycast` _asthird_person_character)
  (bind _output_get (set `self.SpawnDragonLoc` (+ (* (`SceneComponent.GetForwardVector` (`Actor.RootComponent` (`GameplayStatics.GetPlayerCharacter` 0))) 1000.0) (`self.K2_GetActorLocation` _asthird_person_character))))
  (bind (_returnvalue_roll _returnvalue_pitch _returnvalue_yaw) (`KismetMathLibrary.BreakRotator` (`KismetMathLibrary.Conv_VectorToRotator` (`/Game/GameMechanics/Character/ThirdPersonCharacter.CamRay` _asthird_person_character))))
  (bind _returnvalue (`|SpawnActorFromClass` "/Game/GameMechanics/Dragon_Ultimate/BP_UltDDragon.BP_UltDDragon_C" (`KismetMathLibrary.MakeTransform` _output_get (`KismetMathLibrary.MakeRotator` _returnvalue_roll _returnvalue_pitch _returnvalue_yaw)) "Undefined" "OverrideRootScale" null null))
  (`/Game/GameMechanics/Dragon_Ultimate/BP_UltDDragon.UltiCalled` _returnvalue))

(fn `UserConstructionScript`)